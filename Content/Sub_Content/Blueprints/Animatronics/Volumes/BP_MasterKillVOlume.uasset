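; Master kill volume for animatronics that times how long the player has been out of its sphere, with empty hooks for the response.
; End overlap by BP_DemoCharacter stamps real time and opens a Tick-fed gate; begin overlap closes it, despite comments stating the reverse.
; While open, it calls InVolumeCountdow each frame, plus OnVolumeTimeComplete every frame once TimerLength is exceeded.
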(event OnComponentBeginOverlap(SphereCollision)
  (params (OverlappedComponent :type Primitive%20Component%20Object%20Reference) (OtherActor :type Actor%20Object%20Reference) (OtherComp :type Primitive%20Component%20Object%20Reference) (OtherBodyIndex :type Integer) (bFromSweep :type Boolean) (SweepResult :type Hit%20Result%20Structure%20%28by%20ref%29))
  ;[1 0.5391 0] Check when player ends overlap and close gate
  (Utilities|Casting|CastToBP_DemoCharacter OtherActor)
  (Utilities|FlowControl|Gate true) ; enters at Close
)

(event OnComponentEndOverlap(SphereCollision)
  (params (OverlappedComponent :type Primitive%20Component%20Object%20Reference) (OtherActor :type Actor%20Object%20Reference) (OtherComp :type Primitive%20Component%20Object%20Reference) (OtherBodyIndex :type Integer))
  ;[1 0.9375 0] Check when player begins overlap and set time stamp, open gate
  (Utilities|Casting|CastToBP_DemoCharacter OtherActor)
  (Variables|Default|SetTimerStamp (Utilities|Time|GetRealTimeSeconds))
  (Utilities|FlowControl|Gate true) ; enters at Open
)

(event EventBeginPlay)

(event EventTick
  (params (DeltaSeconds :type Float%20%28single-precision%29))
  (Utilities|FlowControl|Gate true
    (:Exit
      ;[0.7813 0 1] Compare to Timer Length and Return True when met
      (CallFunction|InVolumeCountdow)
      (if (> (- (Utilities|Time|GetRealTimeSeconds) (Variables|Default|GetTimerStamp)) (Variables|Default|GetTimerLength))
        (CallFunction|OnVolumeTimeComplete)))))

(fn ConstructionScript)

(fn InVolumeCountdow
  (return))

(fn OnVolumeTimeComplete
  (return))
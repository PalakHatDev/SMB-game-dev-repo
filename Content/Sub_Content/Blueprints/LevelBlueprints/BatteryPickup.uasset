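; BatteryPickup is a level pickup that adds one battery to the player's total when BP_DemoCharacter overlaps its box.
; A DoOnce limits it to a single collection, which increments TotalBatteries in the BP_SnapSave_GameInstance save data.
; It then posts a Wwise flashlight click event on the controller, swaps the mesh for a Niagara effect and destroys itself after a short delay.
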(event OnComponentBeginOverlap(Box)
  (params (OverlappedComponent :type Primitive%20Component%20Object%20Reference) (OtherActor :type Actor%20Object%20Reference) (OtherComp :type Primitive%20Component%20Object%20Reference) (OtherBodyIndex :type Integer) (bFromSweep :type Boolean) (SweepResult :type Hit%20Result%20Structure%20%28by%20ref%29))
  (Utilities|Casting|CastToBP_DemoCharacter OtherActor)
  (Utilities|FlowControl|DoOnce false
    (:Completed
      (Math|Integer|IncrementInt (Variables|/Game/SnapSaveCamera/Blueprints/BP_SaveGame.BP_SaveGame_C|GetTotalBatteries (Variables|/Game/SnapSaveCamera/Blueprints/BP_SnapSave_GameInstance.BP_SnapSave_GameInstance_C|GetSaveData (.AsBP%20Snap%20Save%20Game%20Instance (Utilities|Casting|CastToBP_SnapSave_GameInstance (Game|GetGameInstance)))))
        (:%20%20
          (Class|AkGameplayStatics|PostEvent "/Game/Resources/WwiseAudio/Events/Default_Work_Unit/Player/FlashlightClicks_Play.FlashlightClicks_Play" (Pawn|GetController))
          (Development|SetHiddeninGame (Variables|Default|GetStaticMesh) true false)
          (Development|SetHiddeninGame (Variables|Default|GetNiagara) false false)
          (Utilities|FlowControl|Delay 0.5)
          (Actor|DestroyActor))))))

(event EventBeginPlay)

(event Collision|EventActorBeginOverlap
  (params (OtherActor :type Actor%20Object%20Reference)))

(event EventTick
  (params (DeltaSeconds :type Float%20%28single-precision%29)))

(fn ConstructionScript)
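; Exit door actor that swings open for the player character at a set progress stage and leads to the Lake level.
; Box overlap begin and end both check the progress code; on a match, they free two physics constraints' swing limits and push Door with an impulse.
; A separate Exit trigger opens the Lake level when the player character enters it, without checking progress.
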(event OnComponentBeginOverlap(Box)
  (params (OverlappedComponent :type Primitive%20Component%20Object%20Reference) (OtherActor :type Actor%20Object%20Reference) (OtherComp :type Primitive%20Component%20Object%20Reference) (OtherBodyIndex :type Integer) (bFromSweep :type Boolean) (SweepResult :type Hit%20Result%20Structure%20%28by%20ref%29))
  (Utilities|Casting|CastToBP_DemoCharacter OtherActor)
  (if (== (|GetProgressCode) 2)
    (Class|PhysicsConstraintComponent|SetAngularSwing1Limit (Variables|Default|GetPhysicsConstraint) "ACM_Free" 65.0)
    (Class|PhysicsConstraintComponent|SetAngularSwing1Limit (Variables|Default|GetPhysicsConstraint1) "ACM_Free" 65.0)
    (Physics|AddImpulse (Variables|Default|GetDoor) (Math|Vector|MakeVector 1e+03 0.0 0.0) "None" true)))

(event OnComponentEndOverlap(Box)
  (params (OverlappedComponent :type Primitive%20Component%20Object%20Reference) (OtherActor :type Actor%20Object%20Reference) (OtherComp :type Primitive%20Component%20Object%20Reference) (OtherBodyIndex :type Integer))
  (Utilities|Casting|CastToBP_DemoCharacter OtherActor)
  (if (== (|GetProgressCode) 2)
    (Class|PhysicsConstraintComponent|SetAngularSwing1Limit (Variables|Default|GetPhysicsConstraint) "ACM_Free" 65.0)
    (Class|PhysicsConstraintComponent|SetAngularSwing1Limit (Variables|Default|GetPhysicsConstraint1) "ACM_Free" 65.0)
    (Physics|AddImpulse (Variables|Default|GetDoor) (Math|Vector|MakeVector 1e+03 0.0 0.0) "None" true)))

(event OnComponentBeginOverlap(Exit)
  (params (OverlappedComponent :type Primitive%20Component%20Object%20Reference) (OtherActor :type Actor%20Object%20Reference) (OtherComp :type Primitive%20Component%20Object%20Reference) (OtherBodyIndex :type Integer) (bFromSweep :type Boolean) (SweepResult :type Hit%20Result%20Structure%20%28by%20ref%29))
  (Utilities|Casting|CastToBP_DemoCharacter OtherActor)
  (Game|OpenLevel(byName) "Lake"))

(event EventBeginPlay)

(event Collision|EventActorBeginOverlap
  (params (OtherActor :type Actor%20Object%20Reference)))

(event EventTick
  (params (DeltaSeconds :type Float%20%28single-precision%29)))

(fn ConstructionScript)
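; A maintenance door that unlocks for the demo character based on a progress code.
; Entering or leaving its box checks the code from a progress function; a value of 1 sets the character's DoorUnlock flag, shows text and gives two physics constraints a limited swing.
; Otherwise it clears the flag and hides the text, leaving the constraints untouched.
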(event OnComponentBeginOverlap(Box)
  (params (OverlappedComponent :type Primitive%20Component%20Object%20Reference) (OtherActor :type Actor%20Object%20Reference) (OtherComp :type Primitive%20Component%20Object%20Reference) (OtherBodyIndex :type Integer) (bFromSweep :type Boolean) (SweepResult :type Hit%20Result%20Structure%20%28by%20ref%29))
  (bind _textrender (Variables|Default|GetTextRender))
  (bind _asbp_demo_character (Utilities|Casting|CastToBP_DemoCharacter OtherActor))
  (if (== (Variables|/Game/SnapSaveCamera/Blueprints/BP_SaveGame.BP_SaveGame_C|GetProgressCode (|SaveGameStateProgressUpdate_2_2_2)) 1)
    (Variables|/Game/Sub_Content/Blueprints/Char_BP/BP_DemoCharacter.BP_DemoCharacter_C|SetDoorUnlock _asbp_demo_character true)
    (Rendering|SetVisibility _textrender true false)
    (Class|PhysicsConstraintComponent|SetAngularSwing1Limit (Variables|Default|GetPhysicsConstraint) "ACM_Limited" 65.0)
    (Class|PhysicsConstraintComponent|SetAngularSwing1Limit (Variables|Default|GetPhysicsConstraint1) "ACM_Limited" 65.0)
    (else
      (Variables|/Game/Sub_Content/Blueprints/Char_BP/BP_DemoCharacter.BP_DemoCharacter_C|SetDoorUnlock _asbp_demo_character false)
      (Rendering|SetVisibility _textrender false false))))

(event OnComponentEndOverlap(Box)
  (params (OverlappedComponent :type Primitive%20Component%20Object%20Reference) (OtherActor :type Actor%20Object%20Reference) (OtherComp :type Primitive%20Component%20Object%20Reference) (OtherBodyIndex :type Integer))
  (bind _textrender (Variables|Default|GetTextRender))
  (Utilities|Casting|CastToBP_DemoCharacter OtherActor)
  (if (== (Variables|/Game/SnapSaveCamera/Blueprints/BP_SaveGame.BP_SaveGame_C|GetProgressCode (|SaveGameStateProgressUpdate_2_2_2)) 1)
    (Variables|/Game/Sub_Content/Blueprints/Char_BP/BP_DemoCharacter.BP_DemoCharacter_C|SetDoorUnlock (stale OnComponentBeginOverlap(Box) _asbp_demo_character) true)
    (Rendering|SetVisibility _textrender true false)
    (Class|PhysicsConstraintComponent|SetAngularSwing1Limit (Variables|Default|GetPhysicsConstraint) "ACM_Limited" 65.0)
    (Class|PhysicsConstraintComponent|SetAngularSwing1Limit (Variables|Default|GetPhysicsConstraint1) "ACM_Limited" 65.0)
    (else
      (Variables|/Game/Sub_Content/Blueprints/Char_BP/BP_DemoCharacter.BP_DemoCharacter_C|SetDoorUnlock (stale OnComponentBeginOverlap(Box) _asbp_demo_character) false)
      (Rendering|SetVisibility _textrender false false))))

(event EventBeginPlay)

(event Collision|EventActorBeginOverlap
  (params (OtherActor :type Actor%20Object%20Reference)))

(event EventTick
  (params (DeltaSeconds :type Float%20%28single-precision%29)))

(fn ConstructionScript)
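; Boat mover that carries its actor along a path of Movepoint waypoints after a PlayerInteract signal from the cutscene handler.
; BeginPlay gathers Movepoints matching the actor's tags, and after a short delay a timeline interpolates the root between stored position and current target.
; Each finished leg advances a hardcoded-limit index, runs point triggers (only a debug print), and eases rotation toward the next point before replaying unless already there.
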(event EventBeginPlay
  ;[0.1484 1 0] Parse Points
  (for _array_element (Variables|Actor|GetTags)
    (bind _outactors (Actor|GetAllActorsOfClasswithTag "/Game/Sub_Content/Blueprints/Animatronics/JawsLogic/movepoint.movepoint_C" _array_element))
    (Utilities|Array|AppendArray (Variables|Default|GetOut%20Actors) _outactors)
    (Variables|Default|SetStoredPosNode (Transformation|GetSocketLocation (Variables|Default|GetDefaultSceneRoot) "None")) ; Store Intiail Position
  ))

(event Collision|EventActorBeginOverlap
  (params (OtherActor :type Actor%20Object%20Reference)))

(event EventPlayerInteract
  (params (Character :type BP%20Demo%20Character%20Object%20Reference))
  (bind _out_actors (Variables|Default|GetOut%20Actors))
  (bind _defaultsceneroot (Variables|Default|GetDefaultSceneRoot))
  (bind _returnvalue (Transformation|GetSocketLocation _defaultsceneroot "None"))
  (bind _returnvalue_2 (|GetCurrentTargetLocation _out_actors))
  ;[1 0 0.6562] Signal Recived From Cutscene Handler
  (Utilities|FlowControl|Delay 2.0)
  ;[0 1 0.9531] LocationMover
  (bind _boatmovement (Timeline|Timeline_1 PlayFromStart)
    (:Update
      (Transformation|SetWorldLocation _defaultsceneroot (CallFunction|Vector3LocMapRange (Variables|Default|GetStoredPosNode) _returnvalue_2 _boatmovement) false false))
    (:Finished
      (Utilities|FlowControl|Sequence
        (:then_0
          (bind _result (Math|Integer|IncrementInt (Variables|Default|GetCurrentTarget))
            (:%20%20
              (if (>= 9 _result)
                (CallFunction|ParsePointTriggers _result)
                (Variables|Default|SetStoredPosNode _returnvalue)
                (if (not (Utilities|Operators|EqualEqual _returnvalue_2 _returnvalue 4e+01))
                  (|PauseRotateBoat _defaultsceneroot _returnvalue_2 _defaultsceneroot _returnvalue
                    (:Finished
                      (Timeline|Timeline_1 PlayFromStart))))))))
        (:then_1
          (Timeline|Timeline_1 Stop))))))

(fn ConstructionScript)

(fn StopAnim
  (params (ShakeValue :type Float%20%28double-precision%29)))

(fn StopRandomizer)

(fn Vector3LocMapRange
  (params (Starting :type Vector) (Target :type Vector) (DistanceTraveledPer :type Float%20%28double-precision%29))
  (bind (_x _y _z) (Math|Vector|BreakVector Target))
  (bind (_x_2 _y_2 _z_2) (Math|Vector|BreakVector Starting))
  (return (Math|Vector|MakeVector (Math|Float|MapRangeClamped DistanceTraveledPer 0.0 1.0 _x_2 _x) (Math|Float|MapRangeClamped DistanceTraveledPer 0.0 1.0 _y_2 _y) (Math|Float|MapRangeClamped DistanceTraveledPer 0.0 1.0 _z_2 _z))))

(fn ParsePointTriggers
  (params (Selection :type Integer))
  (switch int Selection
    (:Default)
    (:6
      (Development|PrintString "6thPoint"))
    (:7)
    (:8)))

(fn IsInteractable
  (return false))
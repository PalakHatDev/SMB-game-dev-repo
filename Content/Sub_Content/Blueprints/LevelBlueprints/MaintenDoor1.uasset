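; Interactable maintenance door that stays locked, playing a jiggle sound, until the demo character has touched its Box trigger.
; Both begin and end overlap set DoorUnlock to true, and nothing in the graph relocks it.
; Interacting while unlocked plays a Wwise door sound, teleports Cube far away and eases Door through a one-second rotation.
; It also overrides Door's mass to a huge value and disables its physics simulation.
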(event OnComponentEndOverlap(Box)
  (params (OverlappedComponent :type Primitive%20Component%20Object%20Reference) (OtherActor :type Actor%20Object%20Reference) (OtherComp :type Primitive%20Component%20Object%20Reference) (OtherBodyIndex :type Integer))
  (Utilities|Casting|CastToBP_DemoCharacter OtherActor)
  (Variables|Default|SetDoorUnlock true))

(event OnComponentBeginOverlap(Box)
  (params (OverlappedComponent :type Primitive%20Component%20Object%20Reference) (OtherActor :type Actor%20Object%20Reference) (OtherComp :type Primitive%20Component%20Object%20Reference) (OtherBodyIndex :type Integer) (bFromSweep :type Boolean) (SweepResult :type Hit%20Result%20Structure%20%28by%20ref%29))
  (Utilities|Casting|CastToBP_DemoCharacter OtherActor)
  (Variables|Default|SetDoorUnlock true))

(event EventPlayerInteract
  (params (Character :type BP%20Demo%20Character%20Object%20Reference))
  (bind _door (Variables|Default|GetDoor))
  (if (Variables|Default|GetDoorUnlock)
    (Class|PrimitiveComponent|SetMassOverrideinKg _door "None" 5e+06 true)
    (Class|AkGameplayStatics|PostEvent "/Game/Resources/WwiseAudio/Events/Default_Work_Unit/Player/Foley_SFX/PlasticDoor_Play.PlasticDoor_Play" (Game|GetPlayerController 0))
    (Transformation|SetWorldLocation (Variables|Default|GetCube) "100000.000000,100000.000000,100000.000000" false true)
    (Components|MoveComponentTo _door (Variables|/Script/Engine.SceneComponent|GetRelativeLocation _door) "0.000000,200.000000,0.000000" true true 1.0 true)
    (Physics|SetSimulatePhysics (Variables|Default|GetDoor) false)
    (else
      (Audio|PlaySound2D "/Game/Resources/UserGeneratedAssets/PierreAudio/ManualAudioImport/LockJiggle.LockJiggle" 1.0 1.0 0.0 0 0))))

(fn ConstructionScript)

(fn CanInteractEvent
  (return (Variables|Default|GetTrue)))

(fn IsInteractable
  (return true))
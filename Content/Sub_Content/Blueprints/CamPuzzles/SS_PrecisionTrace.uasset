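; SS_PrecisionTrace is a camera puzzle trigger that checks whether the player photographs a specific target from inside its area.
; Overlap opens a Gate and leaving the Box closes it, so the character's photo-taken event only passes inside.
; Each photo runs a tolerance-based RaycastPhoto and compares the pictured object's name to Target.
; A match shows a tooltip and briefly flags BPCSnapSave to use the reserved slot; a miss shows "Try Again".
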(event OnComponentEndOverlap(Box)
  (params (OverlappedComponent :type Primitive%20Component%20Object%20Reference) (OtherActor :type Actor%20Object%20Reference) (OtherComp :type Primitive%20Component%20Object%20Reference) (OtherBodyIndex :type Integer))
  (Utilities|Casting|CastToBP_DemoCharacter OtherActor)
  (Utilities|FlowControl|Gate true) ; enters at Close
)

(event Custom|PhotoTaken
  (Utilities|FlowControl|Gate true
    (:Exit
      (Default|RaycastPhoto (stale Collision|EventActorBeginOverlap _asbp_demo_character) (Variables|Default|GetSphereTraceTolerance))
      (if (Utilities|Enum|Equal(Enum) (Utilities|GetObjectName (Variables|Default|GetTarget)) (Variables|/Game/Sub_Content/Blueprints/Char_BP/BP_DemoCharacter.BP_DemoCharacter_C|GetPicturedObjectName (stale Collision|EventActorBeginOverlap _asbp_demo_character)))
        (|ShowToolTip_2_2_2_2_2_2_2_2 "Photo Taken" 0.5)
        (Variables|/Game/SnapSaveCamera/BPC_SnapSave.BPC_SnapSave_C|SetUseReservedSlot (Variables|/Game/Sub_Content/Blueprints/Char_BP/BP_DemoCharacter.BP_DemoCharacter_C|GetBPC_SnapSave (stale Collision|EventActorBeginOverlap _asbp_demo_character)) true)
        (Variables|/Game/SnapSaveCamera/BPC_SnapSave.BPC_SnapSave_C|SetReservedSlot (Variables|/Game/Sub_Content/Blueprints/Char_BP/BP_DemoCharacter.BP_DemoCharacter_C|GetBPC_SnapSave (stale Collision|EventActorBeginOverlap _asbp_demo_character)) (Variables|Default|GetReservedSlot))
        (Utilities|FlowControl|Delay 0.03)
        (Variables|/Game/SnapSaveCamera/BPC_SnapSave.BPC_SnapSave_C|SetUseReservedSlot (Variables|/Game/Sub_Content/Blueprints/Char_BP/BP_DemoCharacter.BP_DemoCharacter_C|GetBPC_SnapSave (stale Collision|EventActorBeginOverlap _asbp_demo_character)) false)
        (else
          (|ShowToolTip_2_2_2_2_2_2_2_2_2 "Try Again" 0.5))))))

(event EventTick
  (params (DeltaSeconds :type Float%20%28single-precision%29)))

(event EventBeginPlay
  (EventDispatchers|BindEventtoPhotoTaken (.AsBP%20Demo%20Character (Utilities|Casting|CastToBP_DemoCharacter (Game|GetPlayerCharacter 0))) (delegate Custom|PhotoTaken)))

(event Collision|EventActorBeginOverlap
  (params (OtherActor :type Actor%20Object%20Reference))
  (bind _asbp_demo_character (Utilities|Casting|CastToBP_DemoCharacter OtherActor))
  (Utilities|FlowControl|Gate true) ; enters at Open
)

(fn ConstructionScript)
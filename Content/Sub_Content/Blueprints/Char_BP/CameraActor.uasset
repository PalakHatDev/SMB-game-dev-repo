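; CameraActor is an actor that acts as a flash detection volume aligned with the player's view.
; Each Tick it copies the world transform of the BP_DemoCharacter camera onto its root, without sweeping or teleporting.
; Its Cone component sets InFlash on any SharkMover that begins overlapping it and clears the flag when the overlap ends.
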(event OnComponentBeginOverlap(Cone)
  (params (OverlappedComponent :type Primitive%20Component%20Object%20Reference) (OtherActor :type Actor%20Object%20Reference) (OtherComp :type Primitive%20Component%20Object%20Reference) (OtherBodyIndex :type Integer) (bFromSweep :type Boolean) (SweepResult :type Hit%20Result%20Structure%20%28by%20ref%29))
  (bind _asshark_mover (Utilities|Casting|CastToSharkMover OtherActor))
  (Variables|/Game/Sub_Content/Blueprints/Animatronics/JawsLogic/SharkMover.SharkMover_C|SetInFlash? _asshark_mover true))

(event OnComponentEndOverlap(Cone)
  (params (OverlappedComponent :type Primitive%20Component%20Object%20Reference) (OtherActor :type Actor%20Object%20Reference) (OtherComp :type Primitive%20Component%20Object%20Reference) (OtherBodyIndex :type Integer))
  (bind _asshark_mover (Utilities|Casting|CastToSharkMover OtherActor))
  (Variables|/Game/Sub_Content/Blueprints/Animatronics/JawsLogic/SharkMover.SharkMover_C|SetInFlash? _asshark_mover false))

(event EventBeginPlay)

(event Collision|EventActorBeginOverlap
  (params (OtherActor :type Actor%20Object%20Reference)))

(event EventTick
  (params (DeltaSeconds :type Float%20%28single-precision%29))
  (Transformation|SetWorldTransform (Variables|Default|GetDefaultSceneRoot) (Transformation|GetWorldTransform (Variables|/Game/Sub_Content/Blueprints/Char_BP/BP_DemoCharacter.BP_DemoCharacter_C|GetCamera (.AsBP%20Demo%20Character (Utilities|Casting|CastToBP_DemoCharacter (Game|GetPlayerCharacter 0))))) false false))

(fn ConstructionScript)
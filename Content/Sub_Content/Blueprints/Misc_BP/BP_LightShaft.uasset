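; BP_LightShaft is a placeable god ray effect that aligns its light beam with an assigned Sunlight actor.
; Its construction script creates a dynamic instance of M_LightShaft_Inst on GodRayMesh and passes in the sun's forward vector as the beam direction.
; Color, length, texture ratio and texture scale are also fed to the material, and all of this setup is skipped when no Sunlight is assigned.
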(fn ConstructionScript
  (bind _sunlight (Variables|Default|GetSunlight))
  ;[1 1 1] Material Parameters
  (if (not (== _sunlight 0)) ; If a directional light has been assigned, use its rotation to determine the direction of the light beam
    (bind _returnvalue (Rendering|Material|CreateDynamicMaterialInstance (Variables|BP_Godray|GetGodRayMesh) 0 "/Game/Resources/UnrealMarketplaceAssets/ReefKit/Material/Instance_Material/M_LightShaft_Inst.M_LightShaft_Inst" "None" :!class /Script/Engine.PrimitiveComponent))
    (Rendering|Material|SetVectorParameterValue _returnvalue "Direction" (Math|Conversions|ToLinearColor(Vector) (Math|Rotator|GetRotationXVector (Transformation|GetActorRotation _sunlight))) :!class /Script/Engine.MaterialInstanceDynamic)
    (Rendering|Material|SetVectorParameterValue _returnvalue "Color" (Variables|Default|GetColor) :!class /Script/Engine.MaterialInstanceDynamic)
    (Rendering|Material|SetScalarParameterValue _returnvalue "Length" (Variables|Default|GetLength) :!class /Script/Engine.MaterialInstanceDynamic)
    (Rendering|Material|SetScalarParameterValue _returnvalue "Ratio" (Variables|Default|GetTextureRatio) :!class /Script/Engine.MaterialInstanceDynamic)
    (Rendering|Material|SetScalarParameterValue _returnvalue "Scale" (Variables|Default|GetTextureScale) :!class /Script/Engine.MaterialInstanceDynamic)))
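; A placeable light fixture actor that pairs a Light static mesh with a SpotLight, configured entirely in the construction script.
; Exposed variables drive the spotlight's color and intensity.
; A non-zero LightIndex swaps in an alternate fixture mesh and repositions and rotates the spotlight to suit it.
; A dynamic material instance of an emissive parent material tints the mesh with a separate LightEmissive color.
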(event EventBeginPlay)

(event Collision|EventActorBeginOverlap
  (params (OtherActor :type Actor%20Object%20Reference)))

(event EventTick
  (params (DeltaSeconds :type Float%20%28single-precision%29)))

(fn ConstructionScript
  (bind _spotlight (Variables|Default|GetSpotLight))
  (Utilities|FlowControl|Sequence
    (:then_0
      (Rendering|Components|Light|SetLightColor _spotlight (Variables|Default|GetLight%20color) true)
      (Rendering|Components|Light|SetIntensity _spotlight (Variables|Default|GetIntensity)))
    (:then_1
      (if (not (== (Variables|Default|GetLight_index) 0))
        (Components|StaticMesh|SetStaticMesh (Variables|Default|Getlight) "/Game/Resources/UnrealMarketplaceAssets/creepy_birthday_party/assets/lights_1_static_mesh.lights_1_static_mesh")
        (Transformation|SetRelativeLocationAndRotation (Variables|Default|GetSpotLight) "0.000000,73.000000,-64.000000" "0.000000,90.000000,0.000000" false false)))
    (:then_2
      (bind _returnvalue (Rendering|Material|CreateDynamicMaterialInstance (Variables|Default|Getlight) 0 "/Game/Resources/UnrealMarketplaceAssets/creepy_birthday_party/materials/emissive_parent_material.emissive_parent_material" "None" :!class /Script/Engine.PrimitiveComponent))
      (Rendering|Material|SetVectorParameterValue _returnvalue "color" (Variables|Default|GetLight%20emissive) :!class /Script/Engine.MaterialInstanceDynamic))))
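; Photo-capture component (SnapSave) that runs photo mode and a gallery, persisting the player's shots between sessions.
; Taking a photo captures the character's SceneCapture2D to a render target, shows it, and exports a PNG to the Saved directory, using a reserved slot or searching from index 16.
; After a short delay the PNG is re-imported as a texture into the GameInstance's SaveData and saved.
; Initialization reloads saved files into textures.
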(event Custom|Take%20Photo
  (bind _inphotogallery_ (Variables|Booleans|GetInPhotoGallery?))
  (bind _inphotomode_ (Variables|Booleans|GetInPhotoMode?))
  ;[0 0 0] Take Photo
  (bind (_file_path _array_index) (CallFunction|TakePicture _inphotogallery_ _inphotomode_))
  (if _inphotomode_
    (if (not _inphotogallery_)
      (Utilities|FlowControl|Delay 0.2)
      (CallFunction|ImportPhoto _file_path _array_index)
      (SaveGame|SaveGametoSlot (Variables|/Game/SnapSaveCamera/Blueprints/BP_SnapSave_GameInstance.BP_SnapSave_GameInstance_C|GetSaveData (.AsBP%20Snap%20Save%20Game%20Instance (Utilities|Casting|CastToBP_SnapSave_GameInstance (Game|GetGameInstance)))) "SaveGame"))))

(event Custom|Toggle%20PhotoMode
  ;[0 0 0] Toggle Photo Mode
  (CallFunction|TogglePhotoMode))

(event Custom|Toggle%20PhotoGallery
  ;[0 0 0] Toggle Photo Gallery
  (CallFunction|TogglePhotoGallery)
  (SaveGame|SaveGametoSlot (Variables|/Game/SnapSaveCamera/Blueprints/BP_SnapSave_GameInstance.BP_SnapSave_GameInstance_C|GetSaveData (.AsBP%20Snap%20Save%20Game%20Instance (Utilities|Casting|CastToBP_SnapSave_GameInstance (Game|GetGameInstance)))) "SaveGame"))

(event EventBeginPlay
  ;[0 0 0] Begin play + Initialization
  (CallFunction|Initialize)
  (SaveGame|LoadGamefromSlot "SaveGame"))

(fn Initialize
  ;[1 0 0.04687] Replace with your game instance
  (bind _asbp_snap_save_game_instance (Utilities|Casting|CastToBP_SnapSave_GameInstance (Game|GetGameInstance)))
  (bind _output_get (Variables|ProjectReferences|SetGame%20Instance _asbp_snap_save_game_instance))
  (Variables|ProjectReferences|SetSave%20Data (Variables|/Game/SnapSaveCamera/Blueprints/BP_SnapSave_GameInstance.BP_SnapSave_GameInstance_C|GetSaveData _output_get))
  ;[0.6641 0 1] Replace with your character
  (bind _asbp_demo_character (Utilities|Casting|CastToBP_DemoCharacter (Game|GetPlayerCharacter 0)))
  (Variables|PlayerReferences|SetPlayer%20REF _asbp_demo_character)
  (Variables|PlayerReferences|SetPlayerController%20REF (Game|GetPlayerController 0))
  (bind _returnvalue (UserInterface|CreateWidget "/Game/SnapSaveCamera/Widgets/WBP_PhotoMode.WBP_PhotoMode_C"))
  (bind _output_get_2 (Variables|Widgets|SetW_PhotoMode%20REF _returnvalue))
  (Variables|/Script/UMG.Widget|SetVisibility _output_get_2 "Collapsed")
  (UserInterface|Viewport|AddtoViewport _output_get_2 1)
  (Utilities|Array|Resize (Variables|/Game/SnapSaveCamera/Blueprints/BP_SaveGame.BP_SaveGame_C|GetPhotoGalleryData (Variables|ProjectReferences|GetSave%20Data)) (Variables|Integers|GetPhotoSlots))
  (for (_ _array_index) (Variables|/Game/SnapSaveCamera/Blueprints/BP_SaveGame.BP_SaveGame_C|GetPhotoGalleryData (Variables|ProjectReferences|GetSave%20Data))
    (if (not (.free? (Utilities|Array|Get(acopy) (Variables|/Game/SnapSaveCamera/Blueprints/BP_SaveGame.BP_SaveGame_C|GetPhotoGalleryData (Variables|ProjectReferences|GetSave%20Data)) _array_index)))
      (if (Class|BlueprintPathsLibrary|FileExists (.filepath (Utilities|Array|Get(acopy) (Variables|/Game/SnapSaveCamera/Blueprints/BP_SaveGame.BP_SaveGame_C|GetPhotoGalleryData (Variables|ProjectReferences|GetSave%20Data)) _array_index)))
        (bind _returnvalue_2 (Class|KismetRenderingLibrary|ImportFileasTexture2D (.filepath (Utilities|Array|Get(acopy) (Variables|/Game/SnapSaveCamera/Blueprints/BP_SaveGame.BP_SaveGame_C|GetPhotoGalleryData (Variables|ProjectReferences|GetSave%20Data)) _array_index))))
        (Utilities|Array|SetArrayElem (Variables|/Game/SnapSaveCamera/Blueprints/BP_SaveGame.BP_SaveGame_C|GetPhotoGalleryData (Variables|ProjectReferences|GetSave%20Data)) _array_index (Utilities|Struct|MakeF_PhotoEntry (.filepath (Utilities|Array|Get(acopy) (Variables|/Game/SnapSaveCamera/Blueprints/BP_SaveGame.BP_SaveGame_C|GetPhotoGalleryData (Variables|ProjectReferences|GetSave%20Data)) _array_index)) _returnvalue_2 false (.index (Utilities|Array|Get(acopy) (Variables|/Game/SnapSaveCamera/Blueprints/BP_SaveGame.BP_SaveGame_C|GetPhotoGalleryData (Variables|ProjectReferences|GetSave%20Data)) _array_index)) (.photoid (Utilities|Array|Get(acopy) (Variables|/Game/SnapSaveCamera/Blueprints/BP_SaveGame.BP_SaveGame_C|GetPhotoGalleryData (Variables|ProjectReferences|GetSave%20Data)) _array_index))))
        (Variables|Integers|SetCurrent%20Photo%20In%20Gallery (+ (Variables|Integers|GetCurrent%20Photo%20In%20Gallery) 1))))))

(fn TogglePhotoMode
  (bind _w_photomode_ref (Variables|Widgets|GetW_PhotoMode%20REF))
  (if (Variables|Booleans|GetInPhotoMode?)
    (Widget|SetVisibility _w_photomode_ref "Collapsed")
    (Variables|Booleans|SetInPhotoMode? false)
    (else
      (Widget|SetVisibility _w_photomode_ref "Visible")
      (Variables|Booleans|SetInPhotoMode? true))))

(fn TogglePhotoGallery
  (bind _playercontroller_ref (Variables|PlayerReferences|GetPlayerController%20REF))
  (if (Variables|Booleans|GetInPhotoGallery?)
    (Input|SetIgnoreLookInput _playercontroller_ref false)
    (Widget|RemovefromParent (stale _output_get))
    (Variables|Booleans|SetInPhotoGallery? false)
    (Input|SetInputModeGameOnly _playercontroller_ref false)
    (Variables|/Script/Engine.PlayerController|SetbShowMouseCursor _playercontroller_ref false)
    (else
      (Variables|Booleans|SetInPhotoGallery? true)
      (Pawn|Components|CharacterMovement|DisableMovement (Variables|/Script/Engine.Character|GetCharacterMovement (Variables|PlayerReferences|GetPlayer%20REF)))
      (Input|SetIgnoreLookInput _playercontroller_ref true)
      (if (Variables|Default|GetDroppedPhotos)
        _
        (else
          (|SyncDisplay_2)))
      (bind _returnvalue (UserInterface|CreateWidget "/Game/SnapSaveCamera/Widgets/WBP_PhotoGallery.WBP_PhotoGallery_C" 0 (Variables|/Game/SnapSaveCamera/Blueprints/BP_SaveGame.BP_SaveGame_C|GetPhotoGalleryData (Variables|ProjectReferences|GetSave%20Data))))
      (bind _output_get (Variables|Widgets|SetW_PhotoGallery%20REF _returnvalue))
      (UserInterface|Viewport|AddtoViewport _output_get 6)
      (Input|SetInputModeGameandUI _playercontroller_ref 0 "DoNotLock" true false)
      (Variables|/Script/Engine.PlayerController|SetbShowMouseCursor _playercontroller_ref true)))
  (return))

(fn TakePicture
  (params (InPhotoGallery? :type Boolean) (InPhotoMode? :type Boolean))
  (bind _player_ref (Variables|PlayerReferences|GetPlayer%20REF))
  (bind _save_data (Variables|ProjectReferences|GetSave%20Data))
  (bind _reservedslot (Variables|Default|GetReservedSlot))
  (bind _scenecapturecomponent2d (Variables|/Game/Sub_Content/Blueprints/Char_BP/BP_DemoCharacter.BP_DemoCharacter_C|GetSceneCaptureComponent2D _player_ref))
  (bind _photogallerydata (Variables|/Game/SnapSaveCamera/Blueprints/BP_SaveGame.BP_SaveGame_C|GetPhotoGalleryData _save_data))
  (if (not InPhotoGallery?)
    (if InPhotoMode?
      (bind _returnvalue (Rendering|CreateRenderTarget2D 256 256 "RTF_RGBA8" "(R=0.000000,G=0.000000,B=0.000000,A=1.000000)" true))
      (bind _output_get (Variables|/Script/Engine.SceneCaptureComponent2D|SetTextureTarget _scenecapturecomponent2d _returnvalue))
      (Variables|/Script/Engine.TextureRenderTarget|SetTargetGamma _output_get 1.0)
      (bind _returnvalue_2 (UserInterface|CreateWidget "/Game/SnapSaveCamera/Widgets/WBP_PhotoDisplay.WBP_PhotoDisplay_C" 0 _output_get))
      (Rendering|SceneCapture|CaptureScene _scenecapturecomponent2d :!class /Script/Engine.SceneCaptureComponent2D)
      (UserInterface|Viewport|AddtoViewport _returnvalue_2 0)
      (Audio|PlaySound2D "/Game/SnapSaveCamera/Sounds/SC_TakePhoto.SC_TakePhoto" 1.0 1.0 0.0 0 0)
      (if (Variables|Default|GetUseReservedSlot) ; Override Branch
        (bind _returnvalue_3 (|RegisterNewItem_2 _reservedslot (Variables|/Script/Engine.SceneCaptureComponent2D|GetTextureTarget _scenecapturecomponent2d)))
        (return _returnvalue_3 _reservedslot)
        (else
          (bind _array_index (Utilities|Array|ForEachLoopwithBreak _photogallerydata :!label _label)
            (:LoopBody
              (if (.Free? (Utilities|Struct|BreakF_PhotoEntry (Utilities|Array|Get(acopy) _photogallerydata (+ _array_index 16))))
                (goto _label Break)))
            (:Completed
              (if (< (+ _array_index 16) (Variables|Integers|GetPhotoSlots))
                _
                (else
                  (|ResetPhotoAlbum _photogallerydata)
                  (Variables|Integers|SetCurrent%20Photo%20In%20Gallery 0)))
              (bind _returnvalue_4 (|RegisterNewItem (+ _array_index 16) (Variables|/Script/Engine.SceneCaptureComponent2D|GetTextureTarget _scenecapturecomponent2d)))
              (return _returnvalue_4 (+ _array_index 16)))))))))

(fn ImportPhoto
  (params (File%20Path :type String) (Array%20Index :type Integer))
  (bind _save_data (Variables|ProjectReferences|GetSave%20Data))
  (if (Class|BlueprintPathsLibrary|FileExists File%20Path)
    (bind _returnvalue (Class|KismetRenderingLibrary|ImportFileasTexture2D File%20Path))
    (bind _output_get (Variables|/Game/SnapSaveCamera/Blueprints/BP_SaveGame.BP_SaveGame_C|SetPhotosTakenOverall _save_data (+ (Variables|/Game/SnapSaveCamera/Blueprints/BP_SaveGame.BP_SaveGame_C|GetPhotosTakenOverall _save_data) 1)))
    (Utilities|Array|SetArrayElem (Variables|/Game/SnapSaveCamera/Blueprints/BP_SaveGame.BP_SaveGame_C|GetPhotoGalleryData _save_data) Array%20Index (Utilities|Struct|MakeF_PhotoEntry File%20Path _returnvalue false Array%20Index _output_get))
    (Variables|Integers|SetCurrent%20Photo%20In%20Gallery (+ (Variables|Integers|GetCurrent%20Photo%20In%20Gallery) 1))))

(fn RemovePhoto
  (params (Index%20To%20Reset :type Integer))
  (bind _save_data (Variables|ProjectReferences|GetSave%20Data))
  (bind _photogallerydata (Variables|/Game/SnapSaveCamera/Blueprints/BP_SaveGame.BP_SaveGame_C|GetPhotoGalleryData _save_data))
  (bind _output (Utilities|Array|Get(acopy) _photogallerydata Index%20To%20Reset))
  (bind (_filepath _textured2d _free_ _index _photoid) (Utilities|Struct|BreakF_PhotoEntry _output))
  (Utilities|Array|SetArrayElem _photogallerydata _index (Utilities|Struct|MakeF_PhotoEntry _filepath 0 true _index _photoid))
  (return _photogallerydata))
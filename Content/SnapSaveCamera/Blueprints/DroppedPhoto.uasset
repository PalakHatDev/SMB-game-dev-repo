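; DroppedPhoto is a world actor that displays a saved SnapSave camera photo, selected by PhotoID.
; Construction creates a dynamic material for the photo mesh, which BeginPlay or InitializePhoto fills after a short delay with the gallery texture from the game instance's save data.
; Initialization also rewrites the matching display-gallery entry.
; PlayerInteract sets that entry's Free flag to false and destroys the actor, although IsInteractable always returns false.
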(event Custom|InitializePhoto
  (bind _returnvalue (Game|GetGameInstance))
  (bind _photoid (Variables|Default|GetPhotoID))
  (bind _asbp_snap_save_game_instance (Utilities|Casting|CastToBP_SnapSave_GameInstance _returnvalue))
  (bind _savedata (Variables|/Game/SnapSaveCamera/Blueprints/BP_SnapSave_GameInstance.BP_SnapSave_GameInstance_C|GetSaveData _asbp_snap_save_game_instance))
  (bind _displaygallarydata (Variables|/Game/SnapSaveCamera/Blueprints/BP_SaveGame.BP_SaveGame_C|GetDisplayGallaryData _savedata))
  (bind _output (Utilities|Array|Get(acopy) _displaygallarydata _photoid))
  (Utilities|FlowControl|Delay 0.2) ; Problematic Code
  (Rendering|Material|SetTextureParameterValue (Variables|Default|GetPhotoMaterial) "Image" (.textured2d (Utilities|Array|Get(acopy) (Variables|/Game/SnapSaveCamera/Blueprints/BP_SaveGame.BP_SaveGame_C|GetPhotoGalleryData _savedata) _photoid)))
  (Utilities|Array|SetArrayElem _displaygallarydata _photoid (Utilities|Struct|MakeF_PhotoEntry (.filepath _output) (.textured2d _output) true (.index _output) (.photoid _output))))

(event EventBeginPlay
  (bind _returnvalue (Game|GetGameInstance))
  (bind _photoid (Variables|Default|GetPhotoID))
  (bind _asbp_snap_save_game_instance (Utilities|Casting|CastToBP_SnapSave_GameInstance _returnvalue))
  (bind _savedata (Variables|/Game/SnapSaveCamera/Blueprints/BP_SnapSave_GameInstance.BP_SnapSave_GameInstance_C|GetSaveData _asbp_snap_save_game_instance))
  (bind _displaygallarydata (Variables|/Game/SnapSaveCamera/Blueprints/BP_SaveGame.BP_SaveGame_C|GetDisplayGallaryData _savedata))
  (bind _output (Utilities|Array|Get(acopy) _displaygallarydata _photoid))
  (Utilities|FlowControl|Delay 0.2) ; Problematic Code
  (Rendering|Material|SetTextureParameterValue (Variables|Default|GetPhotoMaterial) "Image" (.textured2d (Utilities|Array|Get(acopy) (Variables|/Game/SnapSaveCamera/Blueprints/BP_SaveGame.BP_SaveGame_C|GetPhotoGalleryData _savedata) _photoid)))
  (Utilities|Array|SetArrayElem _displaygallarydata _photoid (Utilities|Struct|MakeF_PhotoEntry (.filepath _output) (.textured2d _output) true (.index _output) (.photoid _output))))

(event Collision|EventActorBeginOverlap
  (params (OtherActor :type Actor%20Object%20Reference)))

(event EventTick
  (params (DeltaSeconds :type Float%20%28single-precision%29)))

(event EventPlayerInteract
  (params (Character :type BP%20Demo%20Character%20Object%20Reference))
  (bind _returnvalue (Game|GetGameInstance))
  (bind _photoid (Variables|Default|GetPhotoID))
  (bind _asbp_snap_save_game_instance (Utilities|Casting|CastToBP_SnapSave_GameInstance _returnvalue))
  (bind _savedata (Variables|/Game/SnapSaveCamera/Blueprints/BP_SnapSave_GameInstance.BP_SnapSave_GameInstance_C|GetSaveData _asbp_snap_save_game_instance))
  (bind _displaygallarydata (Variables|/Game/SnapSaveCamera/Blueprints/BP_SaveGame.BP_SaveGame_C|GetDisplayGallaryData _savedata))
  (bind _output (Utilities|Array|Get(acopy) _displaygallarydata _photoid))
  (Utilities|Array|SetArrayElem _displaygallarydata _photoid (Utilities|Struct|MakeF_PhotoEntry (.filepath _output) (.textured2d _output) false (.index _output) (.photoid _output)))
  (Actor|DestroyActor))

(fn ConstructionScript
  (bind _returnvalue (Rendering|Material|CreateDynamicMaterialInstance (Variables|Default|GetPhoto) 0 "/Game/SnapSaveCamera/Materials/PhotoMaterialBase.PhotoMaterialBase" "None" :!class /Script/Engine.PrimitiveComponent))
  (Variables|Default|SetPhotoMaterial _returnvalue))

(fn IsInteractable
  (return false))
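; Blueprint function library of getters and setters for a retro graphics look.
; Most functions read or write scalar and vector parameters in MPC_RetroGraphics, covering affine mapping, vertex snapping, color quantization, dithering, depth error, clip and draw distances, and distance field light color.
; Screen percentage and upscale smoothing instead go through console variables and commands.
; Several setters clamp their input to safe ranges.
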(fn IsUpscaleSmoothingDisabled
  (bind _returnvalue (Development|GetConsoleVariableIntValue "r.Upscale.Quality"))
  (return (== _returnvalue 0)))

(fn DisableUpscaleSmoothing
  (params (Disabled :type Boolean))
  (Development|ExecuteConsoleCommand 0 (Utilities|String|Append "r.Upscale.Quality " (Utilities|String|ToString(Integer) (Math|Conversions|ToInteger(Boolean) (not Disabled)))) 0)
  (return))

(fn GetScreenPercentage
  (bind _returnvalue (Development|GetConsoleVariableFloatValue "r.ScreenPercentage"))
  (return _returnvalue))

(fn SetScreenPercentage
  (params (Percent :type Float%20%28double-precision%29))
  (Development|ExecuteConsoleCommand 0 (Utilities|String|Append "r.ScreenPercentage " (Utilities|String|ToString(Float) (Math|Float|Clamp(Float) Percent 1e+01 4e+02))) 0)
  (return))

(fn GetNearClipDistance
  (bind _returnvalue (Rendering|Material|GetScalarParameterValue 0 "/Game/Resources/TemporaryAssets/RetroAssets/Materials/MPC_RetroGraphics.MPC_RetroGraphics" "Near Clip Distance" :!class /Script/Engine.KismetMaterialLibrary))
  (return _returnvalue))

(fn SetNearClipDistance
  (params (Distance :type Float%20%28double-precision%29))
  (Rendering|Material|SetScalarParameterValue 0 "/Game/Resources/TemporaryAssets/RetroAssets/Materials/MPC_RetroGraphics.MPC_RetroGraphics" "Near Clip Distance" (Math|Float|Max(Float) Distance 0.0) :!class /Script/Engine.KismetMaterialLibrary)
  (return))

(fn GetDepthError
  (bind _returnvalue (Rendering|Material|GetScalarParameterValue 0 "/Game/Resources/TemporaryAssets/RetroAssets/Materials/MPC_RetroGraphics.MPC_RetroGraphics" "Depth Error Sensitivity" :!class /Script/Engine.KismetMaterialLibrary))
  (bind _returnvalue_2 (Rendering|Material|GetScalarParameterValue 0 "/Game/Resources/TemporaryAssets/RetroAssets/Materials/MPC_RetroGraphics.MPC_RetroGraphics" "Depth Error" :!class /Script/Engine.KismetMaterialLibrary))
  (return _returnvalue_2 _returnvalue))

(fn SetDepthError
  (params (Depth :type Float%20%28double-precision%29) (Sensitivity :type Float%20%28double-precision%29))
  (Rendering|Material|SetScalarParameterValue 0 "/Game/Resources/TemporaryAssets/RetroAssets/Materials/MPC_RetroGraphics.MPC_RetroGraphics" "Depth Error" Depth :!class /Script/Engine.KismetMaterialLibrary)
  (Rendering|Material|SetScalarParameterValue 0 "/Game/Resources/TemporaryAssets/RetroAssets/Materials/MPC_RetroGraphics.MPC_RetroGraphics" "Depth Error Sensitivity" Sensitivity :!class /Script/Engine.KismetMaterialLibrary)
  (return))

(fn IsAffineMappingEnabled
  (bind _returnvalue (Rendering|Material|GetScalarParameterValue 0 "/Game/Resources/TemporaryAssets/RetroAssets/Materials/MPC_RetroGraphics.MPC_RetroGraphics" "Affine Toggle" :!class /Script/Engine.KismetMaterialLibrary))
  (return (Math|Conversions|ToBoolean(Integer) (Math|Float|Round _returnvalue))))

(fn SetAffineMappingEnabled
  (params (Enabled :type Boolean))
  (Rendering|Material|SetScalarParameterValue 0 "/Game/Resources/TemporaryAssets/RetroAssets/Materials/MPC_RetroGraphics.MPC_RetroGraphics" "Affine Toggle" (Math|Conversions|ToFloat(Boolean) Enabled) :!class /Script/Engine.KismetMaterialLibrary)
  (return))

(fn GetVertexSnap
  (bind _returnvalue (Rendering|Material|GetScalarParameterValue 0 "/Game/Resources/TemporaryAssets/RetroAssets/Materials/MPC_RetroGraphics.MPC_RetroGraphics" "Grid Size Y" :!class /Script/Engine.KismetMaterialLibrary))
  (bind _returnvalue_2 (Rendering|Material|GetScalarParameterValue 0 "/Game/Resources/TemporaryAssets/RetroAssets/Materials/MPC_RetroGraphics.MPC_RetroGraphics" "Grid Size X" :!class /Script/Engine.KismetMaterialLibrary))
  (return (Math|Float|Truncate _returnvalue_2) (Math|Float|Truncate _returnvalue)))

(fn SetVertexSnap
  (params (GridSizeX :type Integer) (GridSizeY :type Integer))
  (Rendering|Material|SetScalarParameterValue 0 "/Game/Resources/TemporaryAssets/RetroAssets/Materials/MPC_RetroGraphics.MPC_RetroGraphics" "Grid Size X" (Math|Conversions|ToFloat(Integer) GridSizeX) :!class /Script/Engine.KismetMaterialLibrary)
  (Rendering|Material|SetScalarParameterValue 0 "/Game/Resources/TemporaryAssets/RetroAssets/Materials/MPC_RetroGraphics.MPC_RetroGraphics" "Grid Size Y" (Math|Conversions|ToFloat(Integer) GridSizeY) :!class /Script/Engine.KismetMaterialLibrary)
  (return))

(fn GetColorQuantization
  (bind _returnvalue (Rendering|Material|GetVectorParameterValue 0 "/Game/Resources/TemporaryAssets/RetroAssets/Materials/MPC_RetroGraphics.MPC_RetroGraphics" "RGB Quantize" :!class /Script/Engine.KismetMaterialLibrary))
  (return (.r _returnvalue) (.g _returnvalue) (.b _returnvalue)))

(fn SetColorQuantization
  (params (R :type Float%20%28double-precision%29) (G :type Float%20%28double-precision%29) (B :type Float%20%28double-precision%29))
  (Rendering|Material|SetVectorParameterValue 0 "/Game/Resources/TemporaryAssets/RetroAssets/Materials/MPC_RetroGraphics.MPC_RetroGraphics" "RGB Quantize" (Utilities|Struct|MakeLinearColor R G B 0.0) :!class /Script/Engine.KismetMaterialLibrary)
  (return))

(fn GetDrawDistanceGridSize
  (bind _returnvalue (Rendering|Material|GetScalarParameterValue 0 "/Game/Resources/TemporaryAssets/RetroAssets/Materials/MPC_RetroGraphics.MPC_RetroGraphics" "Draw Distance Grid Size" :!class /Script/Engine.KismetMaterialLibrary))
  (return _returnvalue))

(fn SetDrawDistanceGridSize
  (params (Size :type Float%20%28double-precision%29))
  (Rendering|Material|SetScalarParameterValue 0 "/Game/Resources/TemporaryAssets/RetroAssets/Materials/MPC_RetroGraphics.MPC_RetroGraphics" "Draw Distance Grid Size" (Math|Float|Max(Float) Size 1.0) :!class /Script/Engine.KismetMaterialLibrary)
  (return))

(fn GetDrawDistance
  (bind _returnvalue (Rendering|Material|GetScalarParameterValue 0 "/Game/Resources/TemporaryAssets/RetroAssets/Materials/MPC_RetroGraphics.MPC_RetroGraphics" "Polygon Draw Distance" :!class /Script/Engine.KismetMaterialLibrary))
  (return _returnvalue))

(fn SetDrawDistance
  (params (Distance :type Float%20%28double-precision%29))
  (Rendering|Material|SetScalarParameterValue 0 "/Game/Resources/TemporaryAssets/RetroAssets/Materials/MPC_RetroGraphics.MPC_RetroGraphics" "Polygon Draw Distance" (Math|Float|Max(Float) Distance 0.0) :!class /Script/Engine.KismetMaterialLibrary)
  (return))

(fn SetDitherIntensity
  (params (Intensity :type Float%20%28double-precision%29))
  (Rendering|Material|SetScalarParameterValue 0 "/Game/Resources/TemporaryAssets/RetroAssets/Materials/MPC_RetroGraphics.MPC_RetroGraphics" "Dither Intensity" Intensity :!class /Script/Engine.KismetMaterialLibrary)
  (return))

(fn GetDistanceFieldLightColor
  (bind _returnvalue (Rendering|Material|GetVectorParameterValue 0 "/Game/Resources/TemporaryAssets/RetroAssets/Materials/MPC_RetroGraphics.MPC_RetroGraphics" "DF Color" :!class /Script/Engine.KismetMaterialLibrary))
  (return _returnvalue))

(fn SetDistanceFieldLightColor
  (params (Color :type Linear%20Color%20Structure :default "(R=1.000000,G=1.000000,B=1.000000,A=1.000000)"))
  (Rendering|Material|SetVectorParameterValue 0 "/Game/Resources/TemporaryAssets/RetroAssets/Materials/MPC_RetroGraphics.MPC_RetroGraphics" "DF Color" Color :!class /Script/Engine.KismetMaterialLibrary)
  (return))

(fn GetDitherIntensity
  (bind _returnvalue (Rendering|Material|GetScalarParameterValue 0 "/Game/Resources/TemporaryAssets/RetroAssets/Materials/MPC_RetroGraphics.MPC_RetroGraphics" "Dither Intensity" :!class /Script/Engine.KismetMaterialLibrary))
  (return _returnvalue))
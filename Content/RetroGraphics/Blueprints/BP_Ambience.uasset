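; Ambience actor for the retro graphics look, controlling global light, shade color and fog through MPC_RetroGraphics, with the actor's rotation setting light direction.
; On construction and BeginPlay it pushes all parameters and assigns a legacy or newer post-process material instance.
; It also draws a 4x4 dither matrix into a render target pixel by pixel when dither intensity is nonzero.
; Setter functions update individual collection parameters at runtime, most clamping their inputs.
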(event EventBeginPlay
  (CallFunction|InitializeParameters)
  (CallFunction|DrawMatrixValuestoRT))

(fn ConstructionScript
  (CallFunction|InitializeParameters)
  (CallFunction|DrawMatrixValuestoRT))

(fn SetLightIntensity
  (params (Intensity :type Float%20%28double-precision%29))
  (bind _color (Variables|Settings|Lighting|GetColor))
  (bind _output_get (Variables|Settings|Lighting|SetIntensity (Math|Float|Max(Float) Intensity 0.0)))
  (Rendering|Material|SetVectorParameterValue "/Game/Resources/TemporaryAssets/RetroAssets/Materials/MPC_RetroGraphics.MPC_RetroGraphics" "Global Light Color" (Utilities|Struct|MakeLinearColor (.r _color) (.g _color) (.b _color) _output_get) :!class /Script/Engine.KismetMaterialLibrary)
  (return))

(fn SetLightColor
  (params (Color :type Linear%20Color%20Structure))
  (bind _output_get (Variables|Settings|Lighting|SetColor (Utilities|Struct|MakeLinearColor (Math|Float|Clamp(Float) (.r Color)) (Math|Float|Clamp(Float) (.g Color)) (Math|Float|Clamp(Float) (.b Color)) 1.0)))
  (Rendering|Material|SetVectorParameterValue "/Game/Resources/TemporaryAssets/RetroAssets/Materials/MPC_RetroGraphics.MPC_RetroGraphics" "Global Light Color" (Utilities|Struct|MakeLinearColor (.r _output_get) (.g _output_get) (.b _output_get) (Variables|Settings|Lighting|GetIntensity)) :!class /Script/Engine.KismetMaterialLibrary)
  (return))

(fn SetVertexNormalInfluence
  (params (Influence :type Float%20%28double-precision%29))
  (bind _output_get (Variables|Settings|Lighting|SetVertexNormalInfluence (Math|Float|Clamp(Float) Influence)))
  (Rendering|Material|SetScalarParameterValue "/Game/Resources/TemporaryAssets/RetroAssets/Materials/MPC_RetroGraphics.MPC_RetroGraphics" "Global Light Dot" _output_get :!class /Script/Engine.KismetMaterialLibrary)
  (return))

(fn SetLightRotation
  (params (Rotation :type Rotator))
  (Transformation|SetActorRotation Rotation)
  (Rendering|Material|SetVectorParameterValue "/Game/Resources/TemporaryAssets/RetroAssets/Materials/MPC_RetroGraphics.MPC_RetroGraphics" "Global Light Direction" (Math|Conversions|ToLinearColor(Vector) (Math|Vector|NegateVector (Transformation|GetActorForwardVector))) :!class /Script/Engine.KismetMaterialLibrary)
  (return))

(fn SetFogColor
  (params (Color :type Linear%20Color%20Structure))
  (bind _output_get (Variables|Settings|Fog|SetFogColor (Utilities|Struct|MakeLinearColor (Math|Float|Clamp(Float) (.r Color)) (Math|Float|Clamp(Float) (.g Color)) (Math|Float|Clamp(Float) (.b Color)) (Variables|Settings|Fog|GetFogDensity))))
  (Rendering|Material|SetVectorParameterValue "/Game/Resources/TemporaryAssets/RetroAssets/Materials/MPC_RetroGraphics.MPC_RetroGraphics" "Fog RGBA" _output_get :!class /Script/Engine.KismetMaterialLibrary)
  (return))

(fn SetFogDensity
  (params (Density :type Float%20%28double-precision%29))
  (bind _fogcolor (Variables|Settings|Fog|GetFogColor))
  (bind _output_get (Variables|Settings|Fog|SetFogDensity (Math|Float|Clamp(Float) Density)))
  (Rendering|Material|SetVectorParameterValue "/Game/Resources/TemporaryAssets/RetroAssets/Materials/MPC_RetroGraphics.MPC_RetroGraphics" "Fog RGBA" (Utilities|Struct|MakeLinearColor (.r _fogcolor) (.g _fogcolor) (.b _fogcolor) _output_get) :!class /Script/Engine.KismetMaterialLibrary)
  (return))

(fn SetFogStartDistance
  (params (FogStartDistance :type Float%20%28double-precision%29))
  (bind _output_get (Variables|Settings|Fog|SetFogStartDistance FogStartDistance))
  (Rendering|Material|SetScalarParameterValue "/Game/Resources/TemporaryAssets/RetroAssets/Materials/MPC_RetroGraphics.MPC_RetroGraphics" "Fog Start Distance" _output_get :!class /Script/Engine.KismetMaterialLibrary)
  (return))

(fn SetFogFadeLength
  (params (Length :type Float%20%28double-precision%29))
  (bind _output_get (Variables|Settings|Fog|SetFogFadeLength (Math|Float|Max(Float) Length 0.0)))
  (Rendering|Material|SetScalarParameterValue "/Game/Resources/TemporaryAssets/RetroAssets/Materials/MPC_RetroGraphics.MPC_RetroGraphics" "Fog Fade Length" _output_get :!class /Script/Engine.KismetMaterialLibrary)
  (return))

(fn SetFogHeightOffset
  (params (Offset :type Float%20%28double-precision%29))
  (bind _output_get (Variables|Settings|Fog|SetFogHeightOffset Offset))
  (Rendering|Material|SetScalarParameterValue "/Game/Resources/TemporaryAssets/RetroAssets/Materials/MPC_RetroGraphics.MPC_RetroGraphics" "Fog Height Offset" _output_get :!class /Script/Engine.KismetMaterialLibrary)
  (return))

(fn SetFogHeightFadeLength
  (params (Length :type Float%20%28double-precision%29))
  (bind _output_get (Variables|Settings|Fog|SetFogHeightFadeLength Length))
  (Rendering|Material|SetScalarParameterValue "/Game/Resources/TemporaryAssets/RetroAssets/Materials/MPC_RetroGraphics.MPC_RetroGraphics" "Fog Height Fade Length" _output_get :!class /Script/Engine.KismetMaterialLibrary)
  (return))

(fn InitializeParameters
  (bind _fogcolor (Variables|Settings|Fog|GetFogColor))
  (bind _color (Variables|Settings|Lighting|GetColor))
  (Utilities|FlowControl|Sequence
    (:then_0
      (Rendering|Material|SetVectorParameterValue "/Game/Resources/TemporaryAssets/RetroAssets/Materials/MPC_RetroGraphics.MPC_RetroGraphics" "Global Light Direction" (Math|Conversions|ToLinearColor(Vector) (Math|Vector|NegateVector (Transformation|GetActorForwardVector))) :!class /Script/Engine.KismetMaterialLibrary)
      (Rendering|Material|SetVectorParameterValue "/Game/Resources/TemporaryAssets/RetroAssets/Materials/MPC_RetroGraphics.MPC_RetroGraphics" "Global Light Color" (Utilities|Struct|MakeLinearColor (.r _color) (.g _color) (.b _color) (Variables|Settings|Lighting|GetIntensity)) :!class /Script/Engine.KismetMaterialLibrary)
      (Rendering|Material|SetVectorParameterValue "/Game/Resources/TemporaryAssets/RetroAssets/Materials/MPC_RetroGraphics.MPC_RetroGraphics" "Global Shade Color" (Variables|Settings|Lighting|GetShadeColor) :!class /Script/Engine.KismetMaterialLibrary)
      (Rendering|Material|SetScalarParameterValue "/Game/Resources/TemporaryAssets/RetroAssets/Materials/MPC_RetroGraphics.MPC_RetroGraphics" "Global Light Dot" (Variables|Settings|Lighting|GetVertexNormalInfluence) :!class /Script/Engine.KismetMaterialLibrary)
      (Rendering|Material|SetScalarParameterValue "/Game/Resources/TemporaryAssets/RetroAssets/Materials/MPC_RetroGraphics.MPC_RetroGraphics" "Fog Start Distance" (Variables|Settings|Fog|GetFogStartDistance) :!class /Script/Engine.KismetMaterialLibrary)
      (Rendering|Material|SetScalarParameterValue "/Game/Resources/TemporaryAssets/RetroAssets/Materials/MPC_RetroGraphics.MPC_RetroGraphics" "Fog Fade Length" (Variables|Settings|Fog|GetFogFadeLength) :!class /Script/Engine.KismetMaterialLibrary)
      (Rendering|Material|SetScalarParameterValue "/Game/Resources/TemporaryAssets/RetroAssets/Materials/MPC_RetroGraphics.MPC_RetroGraphics" "Fog Height Offset" (Variables|Settings|Fog|GetFogHeightOffset) :!class /Script/Engine.KismetMaterialLibrary)
      (Rendering|Material|SetScalarParameterValue "/Game/Resources/TemporaryAssets/RetroAssets/Materials/MPC_RetroGraphics.MPC_RetroGraphics" "Fog Height Fade Length" (Variables|Settings|Fog|GetFogHeightFadeLength) :!class /Script/Engine.KismetMaterialLibrary)
      (Rendering|Material|SetVectorParameterValue "/Game/Resources/TemporaryAssets/RetroAssets/Materials/MPC_RetroGraphics.MPC_RetroGraphics" "Fog RGBA" (Utilities|Struct|MakeLinearColor (.r _fogcolor) (.g _fogcolor) (.b _fogcolor) (Variables|Settings|Fog|GetFogDensity)) :!class /Script/Engine.KismetMaterialLibrary)
      (Rendering|Material|SetScalarParameterValue "/Game/Resources/TemporaryAssets/RetroAssets/Materials/MPC_RetroGraphics.MPC_RetroGraphics" "Light Falloff" (Variables|Settings|Lighting|GetFalloff) :!class /Script/Engine.KismetMaterialLibrary)
      (bind _returnvalue (Rendering|Material|CreateDynamicMaterialInstance (select (Variables|Settings|GetUseLegacyPostProcess) "/Game/Resources/TemporaryAssets/RetroAssets/Materials/M_PostProcess.M_PostProcess" "/Game/Resources/TemporaryAssets/RetroAssets/Materials/M_PostProcess_2.M_PostProcess_2") "None" "None" :!class /Script/Engine.KismetMaterialLibrary))
      (bind _output_get (Variables|Default|SetMID_PostProcess _returnvalue))
      (Utilities|Struct|SetmembersinPostProcessSettings (Variables|/Script/Engine.PostProcessComponent|GetSettings (Variables|Default|GetPostProcess)) (Utilities|Struct|MakeWeightedBlendables (Utilities|Array|MakeArray (Utilities|Struct|MakeWeightedBlendable 1.0 _output_get)))))
    (:then_2
      (return))))

(fn SetGlobalShadeColor
  (params (Color :type Linear%20Color%20Structure%20%28by%20ref%29))
  (bind _output_get (Variables|Settings|Lighting|SetShadeColor Color))
  (Rendering|Material|SetVectorParameterValue "/Game/Resources/TemporaryAssets/RetroAssets/Materials/MPC_RetroGraphics.MPC_RetroGraphics" "Global Shade Color" _output_get :!class /Script/Engine.KismetMaterialLibrary)
  (return))

(fn GetShadeColor
  (return (Variables|Settings|Lighting|GetShadeColor)))

(fn SetLightFalloff
  (params (Falloff :type Float%20%28double-precision%29))
  (bind _output_get (Variables|Settings|Lighting|SetFalloff (Math|Float|Clamp(Float) Falloff)))
  (Rendering|Material|SetScalarParameterValue "/Game/Resources/TemporaryAssets/RetroAssets/Materials/MPC_RetroGraphics.MPC_RetroGraphics" "Light Falloff" _output_get :!class /Script/Engine.KismetMaterialLibrary)
  (return))

(fn GetLightFalloff
  (return (Variables|Settings|Lighting|GetFalloff)))

(fn DrawMatrixValuestoRT
  (bind _row_0 (Variables|Settings|Dither4x4|GetRow%200))
  (bind _row_1 (Variables|Settings|Dither4x4|GetRow%201))
  (bind _row_2 (Variables|Settings|Dither4x4|GetRow%202))
  (bind _row_3 (Variables|Settings|Dither4x4|GetRow%203))
  (bind _returnvalue (Rendering|Material|GetScalarParameterValue "/Game/Resources/TemporaryAssets/RetroAssets/Materials/MPC_RetroGraphics.MPC_RetroGraphics" "Dither Intensity" :!class /Script/Engine.KismetMaterialLibrary))
  (if (!= _returnvalue 0.0)
    (bind _rt_dither_matrix (Variables|Default|GetRT%20Dither%20Matrix)
      (:then
        (Rendering|ClearRenderTarget2D _rt_dither_matrix)
        (bind (_canvas _size _context) (Rendering|BeginDrawCanvastoRenderTarget (Variables|Default|GetRT%20Dither%20Matrix)))
        (for (_array_element _array_index) (Utilities|Array|MakeArray (.x _row_0) (.y _row_0) (.z _row_0) (.w _row_0) (.x _row_1) (.y _row_1) (.z _row_1) (.w _row_1) (.x _row_2) (.y _row_2) (.z _row_2) (.w _row_2) (.x _row_3) (.y _row_3) (.z _row_3) (.w _row_3))
          (Canvas|DrawTexture :self _canvas :ScreenPosition (Utilities|1Dto2DIndex _array_index 4) :ScreenSize "(X=1.000000,Y=1.000000)" :CoordinateSize "(X=1.000000,Y=1.000000)" :RenderColor (Math|Conversions|ToLinearColor(Float) _array_element) :BlendMode "BLEND_Opaque" :PivotPoint "(X=0.500000,Y=0.500000)"))
        (Rendering|EndDrawCanvastoRenderTarget _context)
        (return))
      (:else
        _)))
  (return))